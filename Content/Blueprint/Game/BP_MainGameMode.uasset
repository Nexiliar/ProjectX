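; BP_MainGameMode is a game mode that picks player starts by named game phase and handles respawning.
; Initial start selection always looks up the Phase1 player start.
; RespawnPlayerAtPoint asks BP_GameState whether respawn is allowed, maps the returned current phase to one of five start names, and restarts there.
; It always restarts player controller 0, ignoring its NewPlayer input, and returns the success flag.
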(fn `ChoosePlayerStart`
  (params (Player :type "Controller Object Reference"))
  (returns (ReturnValue :type "Actor Object Reference"))
  (return (`self.K2_FindPlayerStart` Player "Phase1")))

(fn `RespawnPlayerAtPoint`
  (params (NewPlayer :type "Controller Object Reference"))
  (returns (Succes :type Boolean))
  (bind _returnvalue (`GameplayStatics.GetPlayerController` 0))
  (bind _asbp_game_state (cast `/Game/Blueprint/Game/BP_GameState` (`GameplayStatics.GetGameState`)))
  (bind (_succes _curretphase) (`/Game/Blueprint/Game/BP_GameState.CanPlayerRespawn` _asbp_game_state))
  (if _succes
    (`self.RestartPlayerAtPlayerStart` _returnvalue (`self.K2_FindPlayerStart` _returnvalue (select `/Game/Blueprint/Game/CheckPoints/E_Phase_Level` _curretphase :`NewEnumerator0` "Phase1" :`NewEnumerator1` "Phase2" :`NewEnumerator2` "Phase3" :`NewEnumerator3` "Phase4" :`NewEnumerator4` "Phase5")))
    (return _succes)
    (else
      (return _succes))))

(fn `UserConstructionScript`)