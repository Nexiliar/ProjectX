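; Player controller that owns the game's main UI and shows the end-game screen.
; On BeginPlay it creates the in-game and main screen widgets, caches the inventory widget and pushes the main sound mix.
; UnPossess unbinds the health bar, while Possess is empty and the widget initialisation code is disconnected.
; WinScreen creates the end-game widget with the win flag and shows the mouse cursor.
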(event `self.ReceiveBeginPlay`
  (`|ExecutionSequence`
    (:`then_0`
      (bind _returnvalue (`|CreateWidget` "/Game/Blueprint/Widget/W_Ingame.W_Ingame_C"))
      (set `self.IngameWidget` _returnvalue)
      (`UserWidget.AddToViewport` _returnvalue 0)
      (`GameplayStatics.PushSoundMixModifier` "/Game/Blueprint/Sounds/Mx_Main.Mx_Main"))
    (:`then_1`
      (bind _returnvalue_2 (`|CreateWidget` "/Game/Blueprint/Widget/Inventory/InventorySystem/W_MainScreenWidget.W_MainScreenWidget_C"))
      (bind _output_get (set `self.MainInventoryIngameWidget` _returnvalue_2))
      (set `self.InventoryWidget` (`/Game/Blueprint/Widget/Inventory/InventorySystem/W_MainScreenWidget.W_Inventory` _output_get))
      (`UserWidget.AddToViewport` _returnvalue_2 0))))

(event `Key|Y`
  (params (Key :type "Key Structure")))

(event `self.ReceiveUnPossess`
  (params (UnpossessedPawn :type "Pawn Object Reference"))
  (bind _ingamewidget (`self.IngameWidget`))
  ;[1 1 1] To Do GameMode player Dead
  (`/Engine/EditorBlueprintResources/StandardMacros.IsValid` _ingamewidget
    (:`Is Valid`
      (`/Game/Blueprint/Widget/Health/W_StatsCharacterBar.UnbindInitWidget` (`/Game/Blueprint/Widget/W_Ingame.W_HealthBar` _ingamewidget)))))

(event `self.ReceivePossess`
  (params (PossessedPawn :type "Pawn Object Reference")))

(fn `UserConstructionScript`)

(fn `WinScreen`
  (params (`Win?` :type Boolean))
  (bind _returnvalue (`|CreateWidget` "/Game/Blueprint/Widget/Menu/W_EndGame.W_EndGame_C" null `Win?`))
  (`UserWidget.AddToViewport` _returnvalue 0)
  (set `PlayerController.bShowMouseCursor` true))