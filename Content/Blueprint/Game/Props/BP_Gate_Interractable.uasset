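; BP_Gate_Interractable is a placeable prop that lets the player character open a linked Gate by pressing a button nearby.
; While a BP_Character overlaps its trigger Box, a looping timer polls the character's IsButtonPressed flag and is cleared when the overlap ends.
; A detected press calls OpenTheDoor on the Gate once, guarded by DoOnce.
; The construction script applies the configurable mesh and box scale.
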(event `self.ReceiveBeginPlay`)

(event `CheckIsButtonPressed`
  (if (`/Game/Blueprint/Character/BP_Character.isButtonPressed` (stale `self.Box.OnComponentBeginOverlap` _asbp_character))
    (`/Engine/EditorBlueprintResources/StandardMacros.DoOnce` false
      (:`Completed`
        (bind _gate (`self.Gate`)
          (:`then`
            (`/Game/Blueprint/Game/Props/BP_SmallGateT.OpenTheDoor` _gate))
          (:`else`))))))

(event `self.Box.OnComponentBeginOverlap`
  (params (OverlappedComponent :type "PrimitiveComponent Object Reference") (OtherActor :type "Actor Object Reference") (OtherComp :type "PrimitiveComponent Object Reference") (OtherBodyIndex :type Integer) (bFromSweep :type Boolean) (SweepResult :type "HitResult Structure (by ref)"))
  (bind _asbp_character (cast `/Game/Blueprint/Character/BP_Character` OtherActor))
  (bind _returnvalue (`KismetSystemLibrary.K2_SetTimerDelegate` (delegate `CheckIsButtonPressed`) 0.1 true))
  (set `self.CheckButtonTimer` _returnvalue))

(event `self.Box.OnComponentEndOverlap`
  (params (OverlappedComponent :type "PrimitiveComponent Object Reference") (OtherActor :type "Actor Object Reference") (OtherComp :type "PrimitiveComponent Object Reference") (OtherBodyIndex :type Integer))
  (cast `/Game/Blueprint/Character/BP_Character` OtherActor)
  (`KismetSystemLibrary.K2_ClearAndInvalidateTimerHandle` (`self.CheckButtonTimer`)))

(fn `UserConstructionScript`
  (`StaticMeshComponent.SetStaticMesh` (`self.StaticMesh`) (`self.Mesh`))
  (`SceneComponent.SetWorldScale3D` (`self.Box`) (`self.BoxScale`)))