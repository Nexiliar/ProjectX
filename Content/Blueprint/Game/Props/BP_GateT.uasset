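; BP_GateT is a sci-fi gate prop that slides its door vertically when a BP_Character enters its trigger, unless it is blocked.
; A timeline drives the door's Z position with sound on opening, then reverses after a configurable delay once the character leaves.
; Available and NotAvailable events toggle the blocked state and turn both top lights green or red.
; The construction script sets the initial light color from IsBlocked.
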(event `self.ReceiveBeginPlay`)

(event `self.In.OnComponentBeginOverlap`
  (params (OverlappedComponent :type "PrimitiveComponent Object Reference") (OtherActor :type "Actor Object Reference") (OtherComp :type "PrimitiveComponent Object Reference") (OtherBodyIndex :type Integer) (bFromSweep :type Boolean) (SweepResult :type "HitResult Structure (by ref)"))
  (bind _door (`self.Door`))
  (bind (_relativelocation_x _relativelocation_y) (`KismetMathLibrary.BreakVector` (`SceneComponent.RelativeLocation` _door)))
  (cast `/Game/Blueprint/Character/BP_Character` OtherActor)
  (if (`self.isBlocked`)
    _
    (elif (not (`self.isOpened`))
      (set `self.isOpened` true)
      (`GameplayStatics.PlaySoundAtLocation` "/Game/FX_Effects/Sounds/Audio/Sci-fi-door-sound-effect_Cue.Sci-fi-door-sound-effect_Cue" (`self.K2_GetActorLocation` self) (struct) 1.0 1.0 0.0 null null null)
      (bind (_direction _dooropenspeed) (`Timeline|DoorOpen` :!label _label)
        (:`Update`
          (`SceneComponent.K2_SetRelativeLocation` _door (`KismetMathLibrary.MakeVector` _relativelocation_x _relativelocation_y _dooropenspeed) true false))))))

(event `self.In.OnComponentEndOverlap`
  (params (OverlappedComponent :type "PrimitiveComponent Object Reference") (OtherActor :type "Actor Object Reference") (OtherComp :type "PrimitiveComponent Object Reference") (OtherBodyIndex :type Integer))
  (cast `/Game/Blueprint/Character/BP_Character` OtherActor)
  (if (`self.isOpened`)
    (`KismetSystemLibrary.Delay` (`self.DelayB4doorClose`))
    (set `self.isOpened` false)
    (goto _label :!via `ReverseFromEnd`)))

(event `Available`
  (set `self.isBlocked` false)
  (`PrimitiveComponent.SetMaterial` (`self.TopLightB`) 2 "/Game/StarterBundle/ModularScifiProps/Materials/MI_Light_Green.MI_Light_Green")
  (`PrimitiveComponent.SetMaterial` (`self.TopLight`) 2 "/Game/StarterBundle/ModularScifiProps/Materials/MI_Light_Green.MI_Light_Green"))

(event `self.ReceiveTick`
  (params (DeltaSeconds :type "Float (single-precision)")))

(event `NotAvailable`
  (set `self.isBlocked` true)
  (`PrimitiveComponent.SetMaterial` (`self.TopLightB`) 2 "/Game/StarterBundle/ModularScifiProps/Materials/MI_Light_Red.MI_Light_Red")
  (`PrimitiveComponent.SetMaterial` (`self.TopLight`) 2 "/Game/StarterBundle/ModularScifiProps/Materials/MI_Light_Red.MI_Light_Red"))

(fn `UserConstructionScript`
  (if (`self.isBlocked`)
    (`PrimitiveComponent.SetMaterial` (`self.TopLight`) 2 "/Game/StarterBundle/ModularScifiProps/Materials/MI_Light_Red.MI_Light_Red")
    (`PrimitiveComponent.SetMaterial` (`self.TopLightB`) 2 "/Game/StarterBundle/ModularScifiProps/Materials/MI_Light_Red.MI_Light_Red")
    (else
      (`PrimitiveComponent.SetMaterial` (`self.TopLight`) 2 "/Game/StarterBundle/ModularScifiProps/Materials/MI_Light_Green.MI_Light_Green")
      (`PrimitiveComponent.SetMaterial` (`self.TopLightB`) 2 "/Game/StarterBundle/ModularScifiProps/Materials/MI_Light_Green.MI_Light_Green"))))