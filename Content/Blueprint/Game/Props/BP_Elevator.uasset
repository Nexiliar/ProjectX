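; BP_Elevator is an elevator prop that makes a single vertical trip when a BP_Character enters its trigger box.
; After a short delay, the ElevClose timeline slides the glass divider along Z to close it.
; A DoOnce then plays the elevator sound and runs the ElevMove timeline, which moves the static mesh along Z with sweep.
; When the move finishes, ElevClose plays in reverse to reopen the divider.
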(event `self.ReceiveBeginPlay`)

(event `self.Box.OnComponentBeginOverlap`
  (params (OverlappedComponent :type "PrimitiveComponent Object Reference") (OtherActor :type "Actor Object Reference") (OtherComp :type "PrimitiveComponent Object Reference") (OtherBodyIndex :type Integer) (bFromSweep :type Boolean) (SweepResult :type "HitResult Structure (by ref)"))
  (bind _sm_glassdivider (`self.SM_GlassDivider`))
  (bind _staticmesh (`self.StaticMesh`))
  (bind (_relativelocation_x _relativelocation_y) (`KismetMathLibrary.BreakVector` (`SceneComponent.RelativeLocation` _sm_glassdivider)))
  (bind (_relativelocation_x_2 _relativelocation_y_2) (`KismetMathLibrary.BreakVector` (`SceneComponent.RelativeLocation` _staticmesh)))
  (cast `/Game/Blueprint/Character/BP_Character` OtherActor)
  (`KismetSystemLibrary.Delay` 1.0)
  (bind (_direction _doorclose) (`Timeline|ElevClose` :!label _label)
    (:`Update`
      (`SceneComponent.K2_SetRelativeLocation` _sm_glassdivider (`KismetMathLibrary.MakeVector` _relativelocation_x _relativelocation_y _doorclose) true false))
    (:`Finished`
      (`/Engine/EditorBlueprintResources/StandardMacros.DoOnce` false
        (:`Completed`
          (`GameplayStatics.PlaySoundAtLocation` "/Game/FX_Effects/Sounds/Audio/Sci-Fi_Elevator_Cue.Sci-Fi_Elevator_Cue" (`self.K2_GetActorLocation`) (struct) 1.0 1.0 0.0 null null null)
          (bind (_direction_2 _movement) (`Timeline|ElevMove`)
            (:`Update`
              (`SceneComponent.K2_SetRelativeLocation` _staticmesh (`KismetMathLibrary.MakeVector` _relativelocation_x_2 _relativelocation_y_2 _movement) true false))
            (:`Finished`
              (goto _label :!via `ReverseFromEnd`))))))))

(fn `UserConstructionScript`)