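; Destructible environment prop that loses health from any damage and destroys itself when its HealthComponent reports death.
; Each health change spawns a BP_DisplayDamageActor at a randomly jittered offset from the prop, initialized with the damage done and current health.
; Radial damage from a ProjectileDefault passes that projectile's effect and the main mesh's physical surface type to AddEffectBySurfaceType.
; AvailableForEffects always returns false.
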(event `self.HealthComponent.OnDead`
  (`self.K2_DestroyActor`))

(event `self.HealthComponent.OnHealthChange`
  (params (Health :type "Float (single-precision)") (Damage :type "Float (single-precision)"))
  (bind _returnvalue (`|SpawnActorFromClass` "/Game/Blueprint/Game/Props/ActorDamage/BP_DisplayDamageActor.BP_DisplayDamageActor_C" (`KismetMathLibrary.MakeTransform` (+ (`self.K2_GetActorLocation`) (+ (`KismetMathLibrary.MakeVector` (`KismetMathLibrary.RandomFloatInRange` -10.0 10.0) (`KismetMathLibrary.RandomFloatInRange` -10.0 100.0)) (`self.Local Point Spawn Health Number`)))) "Undefined" "OverrideRootScale" null null))
  (`/Game/Blueprint/Game/Props/ActorDamage/BP_DisplayDamageActor.InitActor` _returnvalue Damage Health))

(event `self.ReceiveTick`
  (params (DeltaSeconds :type "Float (single-precision)")))

(event `self.ReceiveAnyDamage`
  (params (Damage :type "Float (single-precision)") (DamageType :type "DamageType Object Reference") (InstigatedBy :type "Controller Object Reference") (DamageCauser :type "Actor Object Reference"))
  (`ProjectXHealthComponent.ChangeHealthValue` (`self.HealthComponent`) (* Damage -1.0)))

(event `self.ReceiveRadialDamage`
  (params (DamageReceived :type "Float (single-precision)") (DamageType :type "DamageType Object Reference") (Origin :type "Vector Structure") (HitInfo :type "HitResult Structure (by ref)") (InstigatedBy :type "Controller Object Reference") (DamageCauser :type "Actor Object Reference"))
  (bind _asprojectile_default (cast `ProjectileDefault` DamageCauser))
  (bind (_projectilesetting_projectile _projectilesetting_projectiledamage _projectilesetting_bulletmesh _projectilesetting_projectileicon _projectilesetting_bulletmeshtransform _projectilesetting_bulletfx _projectilesetting_bulletfxtransform _projectilesetting_decalsize _projectilesetting_decallifetime _projectilesetting_projectilelifetime _projectilesetting_projectileinitspeed _projectilesetting_hitdecals _projectilesetting_hitsound _projectilesetting_hitfxs _projectilesetting_effect) (break `ProjectileInfo` (`ProjectileDefault.ProjectileSetting` _asprojectile_default)))
  (`Types.AddEffectBySurfaceType` self _projectilesetting_effect (`PhysicalMaterial.SurfaceType` (`MaterialInterface.GetPhysicalMaterial` (`PrimitiveComponent.GetMaterial` (`self.MainMesh`) 0)))))

(fn `AvailableForEffects`
  (returns (ReturnValue :type Boolean))
  (return false))

(fn `UserConstructionScript`)