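; Small sci-fi sliding gate prop that can be blocked, with two top lights showing red when blocked and green when available.
; OpenTheDoor, only when unblocked, plays a sound and runs a timeline that sets the door's relative Y with sweep.
; CloseTheDoor reverses that timeline from the end, regardless of blocking.
; Available and NotAvailable switch IsBlocked and the light materials, while the construction script applies the initial color.
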(event `OpenTheDoor`
  (bind _door (`self.Door`))
  (bind (_relativelocation_x _relativelocation_y _relativelocation_z) (`KismetMathLibrary.BreakVector` (`SceneComponent.RelativeLocation` _door)))
  (if (not (`self.isBlocked`))
    (`GameplayStatics.PlaySoundAtLocation` "/Game/FX_Effects/Sounds/Audio/Sci-fi_littleDoor_Cue.Sci-fi_littleDoor_Cue" (`self.K2_GetActorLocation`) (struct) 1.0 1.0 0.0 null null null)
    (bind (_direction _dooropenspeed) (`Timeline|DoorOpen` :!label _label)
      (:`Update`
        (`SceneComponent.K2_SetRelativeLocation` _door (`KismetMathLibrary.MakeVector` _relativelocation_x _dooropenspeed _relativelocation_z) true false)))))

(event `CloseTheDoor`
  (goto _label :!via `ReverseFromEnd`))

(event `self.ReceiveBeginPlay`)

(event `Available`
  (set `self.isBlocked` false)
  (`PrimitiveComponent.SetMaterial` (`self.TopLightB`) 2 "/Game/StarterBundle/ModularScifiProps/Materials/MI_Light_Green.MI_Light_Green")
  (`PrimitiveComponent.SetMaterial` (`self.TopLight`) 2 "/Game/StarterBundle/ModularScifiProps/Materials/MI_Light_Green.MI_Light_Green"))

(event `NotAvailable`
  (set `self.isBlocked` true)
  (`PrimitiveComponent.SetMaterial` (`self.TopLightB`) 2 "/Game/StarterBundle/ModularScifiProps/Materials/MI_Light_Red.MI_Light_Red")
  (`PrimitiveComponent.SetMaterial` (`self.TopLight`) 2 "/Game/StarterBundle/ModularScifiProps/Materials/MI_Light_Red.MI_Light_Red"))

(fn `UserConstructionScript`
  (if (`self.isBlocked`)
    (`PrimitiveComponent.SetMaterial` (`self.TopLight`) 2 "/Game/StarterBundle/ModularScifiProps/Materials/MI_Light_Red.MI_Light_Red")
    (`PrimitiveComponent.SetMaterial` (`self.TopLightB`) 2 "/Game/StarterBundle/ModularScifiProps/Materials/MI_Light_Red.MI_Light_Red")
    (else
      (`PrimitiveComponent.SetMaterial` (`self.TopLight`) 2 "/Game/StarterBundle/ModularScifiProps/Materials/MI_Light_Green.MI_Light_Green")
      (`PrimitiveComponent.SetMaterial` (`self.TopLightB`) 2 "/Game/StarterBundle/ModularScifiProps/Materials/MI_Light_Green.MI_Light_Green"))))