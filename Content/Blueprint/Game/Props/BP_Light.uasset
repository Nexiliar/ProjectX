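; BP_Light is a spotlight prop that either flickers or switches on in response to an event, depending on the NoBlink flag.
; BeginPlay applies the Color variable to the SpotLight, then picks the mode.
; Flicker mode runs a looping timer that hides the light and restores it after a short random delay.
; NoBlink mode instead binds LightOn to the EDLightON dispatcher, which shows the light after a one-second delay.
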(event `LightOn`
  (`KismetSystemLibrary.Delay` 1.0)
  (`SceneComponent.SetVisibility` (`self.SpotLight`) true false))

(event `self.ReceiveBeginPlay`
  (`LightComponent.SetLightColor` (`self.SpotLight`) (`self.Color`) true)
  (if (`self.NoBlink`)
    (add `self.ED_LightON` (delegate `LightOn`))
    (else
      (`KismetSystemLibrary.K2_SetTimerDelegate` (delegate `Blink`) 0.2 true))))

(event `Blink`
  (`SceneComponent.SetVisibility` (`self.SpotLight`) false false)
  (`KismetSystemLibrary.Delay` (`KismetMathLibrary.RandomFloatInRange` 0.1 0.5))
  (`SceneComponent.SetVisibility` (`self.SpotLight`) true false))

(fn `UserConstructionScript`)