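; BP_PickUpActorNew is a pickup item actor that detects characters and removes itself once picked up.
; InitActor applies the static or skeletal weapon mesh from the supplied info, preferring static, destroys the unused component, and prints an error if neither exists.
; Sphere overlap with BP_Character tracks IsOverlapping and passes the character's inventory component to OverlapCharacter, which is empty here.
; PickUpSucces destroys the actor.
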(event `OverlapCharacter`
  (params (ToInventory :type "ProjectXInventoryComponent Object Reference")))

(event `self.ReceiveTick`
  (params (DeltaSeconds :type "Float (single-precision)")))

(event `self.Sphere.OnComponentBeginOverlap`
  (params (OverlappedComponent :type "PrimitiveComponent Object Reference") (OtherActor :type "Actor Object Reference") (OtherComp :type "PrimitiveComponent Object Reference") (OtherBodyIndex :type Integer) (bFromSweep :type Boolean) (SweepResult :type "HitResult Structure (by ref)"))
  (bind _asbp_character (cast `/Game/Blueprint/Character/BP_Character` OtherActor))
  (set `self.IsOverlapping` true)
  (`self.OverlapCharacter` (`ProjectXCharacter.InventoryComponent` _asbp_character)))

(event `self.Sphere.OnComponentEndOverlap`
  (params (OverlappedComponent :type "PrimitiveComponent Object Reference") (OtherActor :type "Actor Object Reference") (OtherComp :type "PrimitiveComponent Object Reference") (OtherBodyIndex :type Integer))
  (cast `/Game/Blueprint/Character/BP_Character` OtherActor)
  (set `self.IsOverlapping` false))

(fn `InitActor`
  (params (InfoActor :type "DropItem Structure"))
  (bind (_weaponstaticmesh _weaponskeletalmesh) (break `DropItem` InfoActor))
  (`/Engine/EditorBlueprintResources/StandardMacros.IsValid` _weaponstaticmesh
    (:`Is Valid`
      (`ActorComponent.K2_DestroyComponent` (`self.SkeletalMesh`))
      (`StaticMeshComponent.SetStaticMesh` (`self.StaticMesh`) _weaponstaticmesh))
    (:`Is Not Valid`
      (`/Engine/EditorBlueprintResources/StandardMacros.IsValid` _weaponskeletalmesh
        (:`Is Valid`
          (`SkinnedMeshComponent.SetSkinnedAssetAndUpdate` (`self.SkeletalMesh`) _weaponskeletalmesh true)
          (`ActorComponent.K2_DestroyComponent` (`self.StaticMesh`)))
        (:`Is Not Valid`
          (`KismetSystemLibrary.PrintString` "ERROR DROP ITEM DONT HAVE ANY MESH"))))))

(fn `PickUpSucces`
  (`self.K2_DestroyActor`))

(fn `UserConstructionScript`)