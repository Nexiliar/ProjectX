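; World pickup actor for a dropped item, showing an info widget while an overlap is reported.
; On BeginPlay, after a short delay, it builds an inventory widget from its slots and item config and caches the player character's InventoryComponent.
; OverlapStartBP toggles the info widget; for backpack items, it also shows or removes the inventory widget if the player has a backpack equipped.
; Data-table setup in the construction script and FullInit is mostly disconnected.
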(event `self.ReceiveBeginPlay`
  (`KismetSystemLibrary.Delay` 0.1)
  (bind _returnvalue (`|CreateWidget` "/Game/Blueprint/Widget/Inventory/InventorySystem/W_PickUpActorInventory.W_PickUpActorInventory_C" (`GameplayStatics.GetPlayerController` 0)))
  (bind _output_get (set `self.PickUpWidget` _returnvalue))
  (bind _returnvalue_2 (`self.GetBackPackSlotsAmount`))
  (`/Game/Blueprint/Widget/Inventory/InventorySystem/W_PickUpActorInventory.InitInventoryOfPickUpActor` _output_get (`self.InventorySlots`) (`self.ItemCFG`) _returnvalue_2)
  (bind _asbp_character (cast `/Game/Blueprint/Character/BP_Character` (`GameplayStatics.GetPlayerCharacter` 0)))
  (set `self.Inventory Component` (`ProjectXCharacter.InventoryComponent` _asbp_character)))

(event `self.OverlapStart_BP`
  (params (isOverlaping :type Boolean))
  (bind _inventory_component (`self.Inventory Component`))
  (bind _pickupwidget (`self.PickUpWidget`))
  (`|ExecutionSequence`
    (:`then_0`
      (`SceneComponent.SetHiddenInGame` (`self.Widget`) (select `bool` isOverlaping :`false` true) false))
    (:`then_1`
      (if (`|EnumEquality` (`.SlotType` (break `EquipmentInfo` (`.EquipmentInfo` (break `Inventory` (`self.ItemCFG`))))) "BackPack")
        (`/Engine/EditorBlueprintResources/StandardMacros.IsValid` _inventory_component
          (:`Is Valid`
            (if (`ProjectXInventoryComponent.isBackPackEquiped` _inventory_component)
              (if isOverlaping
                (`UserWidget.AddToViewport` _pickupwidget 0)
                (else
                  (`/Engine/EditorBlueprintResources/StandardMacros.IsValid` self
                    (:`Is Valid`
                      (`Widget.RemoveFromParent` _pickupwidget))))))))))))

(fn `FullInit`
  (`|GetDataTableRow` "/Game/Tables/DT_Inventory.DT_Inventory" (`self.NameOfTheItem`)))

(fn `UserConstructionScript`)