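; Weapon pickup actor that offers its weapon to a character's inventory on overlap.
; InitActor copies the weapon info from the passed info actor before running the parent initialization.
; On character overlap it calls TryGetWeaponToInventory with that info and triggers the pickup success logic if accepted.
; The failure branch only casts the inventory owner to BP_Character, with no further action.
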(event `self.OverlapCharacter`
  (params (ToInventory :type "ProjectXInventoryComponent Object Reference"))
  (`parent.OverlapCharacter` ToInventory)
  (`ProjectXInventoryComponent.TryGetWeaponToInventory` ToInventory (`self.WeaponInfo`))
  (if true
    (`self.PickUpSucces`)
    (else
      (cast `/Game/Blueprint/Character/BP_Character` (`ActorComponent.GetOwner` ToInventory)))))

(fn `InitActor`
  (params (InfoActor :type "DropItem Structure"))
  (set `self.WeaponInfo` (`.WeaponInfo` (break `DropItem` InfoActor)))
  (`parent.InitActor` InfoActor))

(fn `UserConstructionScript`
  (`parent.UserConstructionScript`))