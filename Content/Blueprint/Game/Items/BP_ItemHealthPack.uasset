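; Health pack item Blueprint that initializes itself on BeginPlay by calling ItemInit with the "Health" key.
; Every Tick it fetches its ItemsInfo struct through ReturnAll and prints name, description, icon, usability, stacking and type as a zero-duration debug string.
; The construction script only calls the parent, and no healing or pickup logic is implemented here.
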(event `self.ReceiveTick`
  (params (DeltaSeconds :type "Float (single-precision)"))
  (bind _inventory (`self.ReturnAll`))
  (bind (_itemname _itemdescription _itemicon _itemmesh _itemcanbeused _itemusetext _itemcanbestacked _amountofitemsinslot _itemtype) (break `ItemsInfo` (`.ItemsInfo` (break `Inventory` _inventory))))
  (`KismetSystemLibrary.PrintString` (`KismetStringLibrary.Concat_StrStr` (`KismetStringLibrary.Conv_NameToString` _itemname) "" (`KismetTextLibrary.Conv_TextToString` _itemdescription) "" (`KismetSystemLibrary.GetDisplayName` _itemicon) "" (`KismetStringLibrary.Conv_BoolToString` _itemcanbeused) "" (`KismetTextLibrary.Conv_TextToString` _itemusetext) "" (`KismetStringLibrary.Conv_BoolToString` _itemcanbestacked) "" (`|GetEnumeratorNameAsString` _itemtype)) true true (struct :`G` 0.66 :`B` 1.0 :`A` 1.0) 0.0))

(event `self.ReceiveBeginPlay`
  (`self.ItemInit` "Health"))

(fn `UserConstructionScript`
  (`parent.UserConstructionScript`))