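; BP_KillScore is an actor component that awards experience when its owner dies.
; DeadOwner passes ExpFromKill to BP_MainGameMode's EnemyKilled, then calls AddExp on player 0's BP_Character.
; A binding to the owner's ProjectXHealthComponent death event is present but disconnected, and BeginPlay is empty, so DeadOwner relies on an outside caller.
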(event `self.ReceiveBeginPlay`)

(event `DeadOwner`
  (bind _asbp_main_game_mode (cast `/Game/Blueprint/Game/BP_MainGameMode` (`GameplayStatics.GetGameMode`)))
  (`/Game/Blueprint/Game/BP_MainGameMode.EnemyKilled` _asbp_main_game_mode (`self.ExpFromKill`))
  (bind _asbp_character (cast `/Game/Blueprint/Character/BP_Character` (`GameplayStatics.GetPlayerCharacter` 0)))
  (`/Game/Blueprint/Character/BP_Character.AddExp` _asbp_character))