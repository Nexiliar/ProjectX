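; BP_ComplexTest is a test character blueprint assembled from modular skeletal mesh parts.
; The construction script makes the soldier body and bag meshes follow the main Mesh through master pose.
; CoordForMove cycles through an array of point actors, returning the next location whenever velocity is zero, wrapping at an invalid entry.
; An unconnected fragment would set the armed flag on the ThirdPerson anim instance.
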(event `self.ReceiveBeginPlay`)

(fn `Coord For Move`
  (returns (PointLocation :type "Vector Structure"))
  (bind _output (`|GetArrayItem` (`self.Point For move`) (`self.Count`)))
  (if (== (`MovementComponent.Velocity` (`self.CharacterMovement`)) (0.0 0.0 0.0))
    (set `self.Count` (+ (`self.Count`) 1))
    (if (not (`KismetSystemLibrary.IsValid` _output))
      (set `self.Count` 0))
    (return (`self.K2_GetActorLocation` _output))))

(fn `UserConstructionScript`
  (`SkinnedMeshComponent.SetLeaderPoseComponent` (`self.6fbx`) (`self.Mesh`) false)
  (`SkinnedMeshComponent.SetLeaderPoseComponent` (`self.Soldier_ru_bags`) (`self.Mesh`) false))