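; AI controller for alien characters that runs the alien behavior tree and feeds it perception results through the blackboard.
; On BeginPlay it starts BT_AI_Alien and sets the initial AI state.
; Perception updates branch by sense: hearing a Player-tagged actor records its location, while other senses set the target upon sighting a player.
; Losing a sensed actor clears the target and saves its location as last known.
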(event `self.ReceiveBeginPlay`
  (`self.RunBehaviorTree` "/Game/Blueprint/Character/Aliens/Common/BT_AI_Alien.BT_AI_Alien")
  (`BlackboardComponent.SetValueAsEnum` (`AIBlueprintHelperLibrary.GetBlackboard` null) "BB_AI_State" 3))

(event `self.AIPerception.OnTargetPerceptionUpdated`
  (params (Actor :type "Actor Object Reference") (Stimulus :type "AIStimulus Structure"))
  (bind _returnvalue (`AIBlueprintHelperLibrary.GetBlackboard` null))
  (bind _returnvalue_2 (`AIBlueprintHelperLibrary.GetBlackboard` null))
  (bind _returnvalue_3 (`AIBlueprintHelperLibrary.GetBlackboard` null))
  (bind _currenttarget (`self.CurrentTarget`))
  (`/Engine/EditorBlueprintResources/StandardMacros.IsValid` Actor
    (:`Is Valid`
      (set `self.CurrentTarget` Actor)
      (bind _returnvalue_4 (`AIPerceptionSystem.GetSenseClassForStimulus` Stimulus))
      (if (== _returnvalue_4 "/Script/AIModule.AISense_Hearing")
        (if (`self.ActorHasTag` (`self.CurrentTarget`) "Player")
          (`BlackboardComponent.SetValueAsVector` _returnvalue_2 "LastTargetVector" (`self.K2_GetActorLocation` (`self.CurrentTarget`)))
          (`BlackboardComponent.SetValueAsBool` _returnvalue_2 "CanHearTarget" true))
        (elif (`.bSuccessfullySensed` (break `AIStimulus` Stimulus))
          ;[1 1 1] To do more
          (if (`self.ActorHasTag` (`self.CurrentTarget`) "Player")
            (`BlackboardComponent.SetValueAsObject` _returnvalue "TargetActor" _currenttarget)
            (`BlackboardComponent.SetValueAsVector` _returnvalue "TargetVector" (`self.K2_GetActorLocation` _currenttarget))
            (`BlackboardComponent.SetValueAsBool` _returnvalue "CanSeeTarget" true))
          (else
            (`/Engine/EditorBlueprintResources/StandardMacros.IsValid` (`self.CurrentTarget`)
              (:`Is Valid`
                (`BlackboardComponent.SetValueAsObject` _returnvalue_3 "TargetActor" null)
                (`BlackboardComponent.SetValueAsVector` _returnvalue_3 "TargetVector" (0.0 0.0 0.0))
                (`BlackboardComponent.SetValueAsBool` _returnvalue_3 "CanSeeTarget" false)
                (`BlackboardComponent.SetValueAsVector` _returnvalue_3 "LastTargetVector" (`self.K2_GetActorLocation` (`self.CurrentTarget`))))
              (:`Is Not Valid`
                (`KismetSystemLibrary.PrintString` "TargetPerciption :: Current target invalid")))))))
    (:`Is Not Valid`
      (set `self.CurrentTarget` null))))

(fn `UserConstructionScript`)