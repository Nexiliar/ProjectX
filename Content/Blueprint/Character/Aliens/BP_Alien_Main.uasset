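; Base alien enemy character with health, light and heavy melee attacks, a scream and death handling.
; Attack montages fire notifies that run a forward sphere trace, applying randomized damage to tagged actors.
; Damage feeds ProjectXHealth, whose death event records the kill, drops an item, plays a montage, then ragdolls the body.
; Screaming locks movement and attacks; death during it defers unpossession, drop and animation until the scream's timer calls Reset.
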(event `ResetOnDead`
  (bind _mesh (`self.Mesh`))
  ;[1 1 1] Dead
  (set `self.bIsDead` true :!label _label)
  (`self.OnDead`)
  (`/Game/Blueprint/ActorComponent/BP_KillScore.DeadOwner` (`self.BP_KillScore`))
  (if (not (`self.isScreaming`))
    (`self.Dead Event`)
    (`/Game/Blueprint/ActorComponent/BP_DropItemComponent.Spawn Item` (`self.BP_DropItemComponent`) (`SceneComponent.K2_GetComponentToWorld` (`self.CapsuleComponent`)))
    (`|PlayMontage` (`self.Mesh`) (`self.DeathAnim`)
      (:`OnCompleted`
        _)
      (:`OnInterrupted`
        _))
    (`PrimitiveComponent.SetSimulatePhysics` _mesh true)
    (`PrimitiveComponent.SetCollisionProfileName` _mesh "PhysicsActor" true)
    (`PrimitiveComponent.SetCollisionResponseToChannel` (`self.CapsuleComponent`) "ECC_Pawn" "ECR_Ignore")))

(event `self.ProjectXHealth.OnDead`
  ;[1 1 1] Dead
  (goto _label))

(event `self.ReceiveTick`
  (params (DeltaSeconds :type "Float (single-precision)")))

(event `self.ReceiveBeginPlay`
  (`ProjectXHealthComponent.SetCurrentMaxHealth` (`self.ProjectXHealth`) (`self.Health`)))

(event `self.ReceiveAnyDamage`
  (params (Damage :type "Float (single-precision)") (DamageType :type "DamageType Object Reference") (InstigatedBy :type "Controller Object Reference") (DamageCauser :type "Actor Object Reference"))
  (if (not (`self.bIsDead`))
    (`ProjectXHealthComponent.ChangeHealthValue` (`self.ProjectXHealth`) (* Damage -1.0))))

(event `self.ReceiveRadialDamage`
  (params (DamageReceived :type "Float (single-precision)") (DamageType :type "DamageType Object Reference") (Origin :type "Vector Structure") (HitInfo :type "HitResult Structure (by ref)") (InstigatedBy :type "Controller Object Reference") (DamageCauser :type "Actor Object Reference"))
  (bind _asprojectile_default (cast `ProjectileDefault` DamageCauser))
  (if (not (`self.bIsDead`))
    (bind (_projectilesetting_projectile _projectilesetting_projectiledamage _projectilesetting_bulletmesh _projectilesetting_projectileicon _projectilesetting_bulletmeshtransform _projectilesetting_bulletfx _projectilesetting_bulletfxtransform _projectilesetting_decalsize _projectilesetting_decallifetime _projectilesetting_projectilelifetime _projectilesetting_projectileinitspeed _projectilesetting_hitdecals _projectilesetting_hitsound _projectilesetting_hitfxs _projectilesetting_effect) (break `ProjectileInfo` (`ProjectileDefault.ProjectileSetting` _asprojectile_default)))
    (`Types.AddEffectBySurfaceType` self _projectilesetting_effect (`PhysicalMaterial.SurfaceType` (`MaterialInterface.GetPhysicalMaterial` (`PrimitiveComponent.GetMaterial` (`self.Mesh`) 0))))))

(event `/Game/Blueprint/Character/Aliens/Common/BPI_MeleeCombat.MeleeAttackHeavy`
  (bind _heavyattackanim (`self.HeavyAttackAnim`))
  (bind _baseheavydamage (`self.BaseHeavyDamage`))
  (`self.SetStateMovement` false)
  (`self.SetStateAttack` false)
  (bind _notifyname (`|PlayMontage` (`self.Mesh`) (`|GetArrayItem` _heavyattackanim (`KismetMathLibrary.RandomInteger` (`KismetArrayLibrary.Array_Length` _heavyattackanim))))
    (:`OnCompleted`
      (`self.SetStateAttack` true :!label _label_2)
      (`self.SetStateMovement` true))
    (:`OnInterrupted`
      (goto _label_2))
    (:`OnNotifyBegin`
      (if (== _notifyname "Attack")
        (`self.MeleeAttackTrace` (`self.HeavyRadius`) (`KismetMathLibrary.RandomFloatInRange` (- _baseheavydamage 5.0) (+ _baseheavydamage 5.0)) (`self.Start Trace`) (`self.End Trace`))))))

(event `/Game/Blueprint/Character/Aliens/Common/BPI_MeleeCombat.MeleeAttackLight`
  (bind _baselightdamage (`self.BaseLightDamage`))
  (`self.SetStateAttack` false)
  (bind _notifyname (`|PlayMontage` (`self.Mesh`) (`self.LightAttackAnim`))
    (:`OnCompleted`
      (`self.SetStateAttack` true :!label _label_3))
    (:`OnInterrupted`
      (goto _label_3))
    (:`OnNotifyBegin`
      (if (== _notifyname "Attack")
        (`self.MeleeAttackTrace` (`self.LightRadius`) (`KismetMathLibrary.RandomFloatInRange` (- _baselightdamage 2.0) (+ _baselightdamage 4.0)) (`self.Start Trace`) (`self.End Trace`))))))

(fn `CanAttack`
  (returns (CanAttack :type Boolean))
  (return (`self.CanAttackPawn`)))

(fn `CanMove`
  (returns (CanMove :type Boolean))
  (return (`self.CanMovePawn`)))

(fn `Dead Event`
  (bind _returnvalue (`self.GetController`))
  (`/Engine/EditorBlueprintResources/StandardMacros.IsValid` _returnvalue
    (:`Is Valid`
      (`Controller.UnPossess` _returnvalue)
      (`self.SetStateMovement` false)
      (`self.SetStateAttack` false)
      (`self.SetLifeSpan` (`self.BodyDIssapearTime`))
      (set `CharacterMovementComponent.MaxWalkSpeed` 0.0 (`self.CharacterMovement`)))))

(fn `Reset`
  (set `self.isScreaming` false)
  (`self.SetStateMovement` true)
  (`self.SetStateAttack` true)
  (set `CharacterMovementComponent.MaxWalkSpeed` 400.0 (`self.CharacterMovement`))
  (if (`self.bIsDead`)
    (`self.ResetOnDead`)))

(fn `Scream`
  (set `self.isScreaming` true)
  (`self.SetStateMovement` false)
  (`self.SetStateAttack` false)
  (bind _returnvalue (`self.PlayAnimMontage` (`self.Scream Animation`)))
  (set `CharacterMovementComponent.MaxWalkSpeed` 0.0 (`self.CharacterMovement`))
  (`KismetSystemLibrary.K2_SetTimer` null "Reset" _returnvalue))

(fn `SetStateAttack`
  (params (CanAttack :type Boolean))
  (set `self.CanAttackPawn` CanAttack))

(fn `SetStateMovement`
  (params (CanMove :type Boolean))
  (set `self.CanMovePawn` CanMove))

(fn `UserConstructionScript`)