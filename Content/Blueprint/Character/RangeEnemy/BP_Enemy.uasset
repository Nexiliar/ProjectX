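; BP_Enemy is an enemy character that patrols a looping list of PointForMove actors and can be damaged and killed.
; Successful AI moves restart RunOverPoint, and CoordForMove advances to the next point when velocity is zero.
; AnyDamage reduces the ProjectXHealth component, whose OnDead drops a collision channel response, zeroes walk speed, notifies BPKillScore and plays the death montage.
; A respawn snippet is unconnected and never runs.
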(event `self.ReceiveBeginPlay`
  (bind _projectxhealth (`self.ProjectXHealth`))
  (`self.RunOverPoint`)
  (`ProjectXHealthComponent.SetCurrentMaxHealth` _projectxhealth 100.0)
  (`ProjectXHealthComponent.SetCurrentHealth` _projectxhealth 100.0))

(event `RunOverPoint`
  (bind _pointlocation (`self.Coord For Move`))
  (`|AIMoveTo` self _pointlocation null
    (:`OnSuccess`
      (`self.RunOverPoint`))))

(event `self.ProjectXHealth.OnDead`
  (`PrimitiveComponent.SetCollisionResponseToChannel` (`self.CapsuleComponent`) "ECC_GameTraceChannel2" "ECR_Ignore")
  (`PrimitiveComponent.SetCollisionResponseToChannel` (`self.Mesh`) "ECC_GameTraceChannel2" "ECR_Ignore")
  (set `CharacterMovementComponent.MaxWalkSpeed` 0.0 (`self.CharacterMovement`))
  (`/Game/Blueprint/ActorComponent/BP_KillScore.DeadOwner` (`self.BP_KillScore`))
  (bind _returnvalue (`self.PlayAnimMontage` "/Game/Blueprint/Character/Mannequin/Animations/AnimStarterPack/AM_Death.AM_Death"))
  (`KismetSystemLibrary.Delay` (- _returnvalue 0.2)))

(event `self.ReceiveAnyDamage`
  (params (Damage :type "Float (single-precision)") (DamageType :type "DamageType Object Reference") (InstigatedBy :type "Controller Object Reference") (DamageCauser :type "Actor Object Reference"))
  (`ProjectXHealthComponent.ChangeHealthValue` (`self.ProjectXHealth`) (* Damage -1.0)))

(event `self.ReceiveTick`
  (params (DeltaSeconds :type "Float (single-precision)")))

(fn `Coord For Move`
  (returns (PointLocation :type "Vector Structure"))
  (bind _output (`|GetArrayItem` (`self.Point For move`) (`self.Count`)))
  (if (== (`MovementComponent.Velocity` (`self.CharacterMovement`)) (0.0 0.0 0.0))
    (set `self.Count` (+ (`self.Count`) 1))
    (if (not (`KismetSystemLibrary.IsValid` _output))
      (set `self.Count` 0))
    (return (`self.K2_GetActorLocation` _output))))

(fn `UserConstructionScript`)