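; Friendly NPC character with a modular male or female body, patrol-point lookup, rifle shooting and health.
; The construction script picks meshes by gender and slaves them to the body mesh via master pose.
; ShootTarget enables burst fire when crouched or aiming and fires along control rotation; damage feeds ProjectXHealth, whose death event plays a montage, then ragdolls.
; BeginPlay is empty, leaving weapon and health setup disconnected; CanMove and CanSit always return false.
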(event `self.ReceiveBeginPlay`)

(event `WeaponInit`
  (bind _returnvalue (`|SpawnActorFromClass` "/Game/Blueprint/Weapons/BP_WeaponDefault_Rifle_v1.BP_WeaponDefault_Rifle_v1_C" (`SceneComponent.GetSocketTransform` (`self.Mesh`) "WeaponSocketNoAim" "RTS_World") "AlwaysSpawn" "OverrideRootScale" null null))
  (bind _output_get (set `self.Weapon` _returnvalue))
  (set `WeaponDefault.WeaponSetting` (`self.WeaponSettings`) (`self.Weapon`))
  (`self.K2_AttachToComponent` _output_get (`self.Mesh`) "WeaponSocketNoAim" "KeepWorld" "KeepWorld" "KeepWorld" false))

(event `/Game/Blueprint/Character/RangeEnemy/BPI_RangeEnemy.ShootTarget`
  (params (FireRate :type "Float (single-precision)"))
  (bind _weapon (`self.Weapon`))
  (if (or (`self.CrouchEnabled`) (`self.AimEnabled`))
    (bind _updatedweaponinfo (`self.ReinitBurst` true))
    (set `self.WeaponSettings` _updatedweaponinfo)
    (elif (`.BurstFire` (break `WeaponInfo` (`self.WeaponSettings`)))
      (bind _updatedweaponinfo_2 (`self.ReinitBurst` false))
      (set `self.WeaponSettings` _updatedweaponinfo_2)))
  (`KismetSystemLibrary.Delay` FireRate)
  (set `WeaponDefault.ShootEndLocation` (+ (`SceneComponent.K2_GetComponentLocation` (`WeaponDefault.ShootLocation` _weapon)) (* (`KismetMathLibrary.GetForwardVector` (`self.GetControlRotation`)) 50.0)) _weapon)
  (`WeaponDefault.Fire` _weapon))

(event `self.ProjectXHealth.OnDead`
  (bind _mesh (`self.Mesh`))
  (set `self.Dead` true)
  (`PrimitiveComponent.SetCollisionResponseToChannel` (`self.CapsuleComponent`) "ECC_GameTraceChannel2" "ECR_Ignore")
  (`PrimitiveComponent.SetCollisionResponseToChannel` (`self.Mesh`) "ECC_GameTraceChannel2" "ECR_Ignore")
  (set `CharacterMovementComponent.MaxWalkSpeed` 0.0 (`self.CharacterMovement`))
  (`|PlayMontage` (`self.Mesh`) "/Game/Blueprint/Character/Mannequin/Animations/AnimStarterPack/AM_Death.AM_Death"
    (:`OnCompleted`
      _)
    (:`OnInterrupted`
      _))
  (`PrimitiveComponent.SetSimulatePhysics` _mesh true)
  (`PrimitiveComponent.SetCollisionProfileName` _mesh "PhysicsActor" true)
  (`PrimitiveComponent.SetCollisionResponseToChannel` (`self.CapsuleComponent`) "ECC_Pawn" "ECR_Ignore"))

(event `self.ReceiveAnyDamage`
  (params (Damage :type "Float (single-precision)") (DamageType :type "DamageType Object Reference") (InstigatedBy :type "Controller Object Reference") (DamageCauser :type "Actor Object Reference"))
  (`ProjectXHealthComponent.ChangeHealthValue` (`self.ProjectXHealth`) (* Damage -1.0)))

(fn `CanMove`
  (returns (Success :type Boolean))
  (return false))

(fn `CanShoot`
  (returns (Success :type Boolean))
  (return (`self.AbleToShoot`)))

(fn `CanSit`
  (returns (Success :type Boolean))
  (return false))

(fn `Coord For Move`
  (returns (PointLocation :type "Vector Structure"))
  (bind _output (`|GetArrayItem` (`self.Point For move`) (`self.Count`)))
  (if (== (`MovementComponent.Velocity` (`self.CharacterMovement`)) (0.0 0.0 0.0))
    (set `self.Count` (+ (`self.Count`) 1))
    (if (not (`KismetSystemLibrary.IsValid` _output))
      (set `self.Count` 0))
    (return (`self.K2_GetActorLocation` _output))))

(fn `Init Outlook`
  (params (Body :type "SkeletalMesh Object Reference") (Head :type "SkeletalMesh Object Reference") (Hair :type "SkeletalMesh Object Reference") (Hands :type "SkeletalMesh Object Reference") (Foot :type "SkeletalMesh Object Reference") (Legs :type "SkeletalMesh Object Reference"))
  (`SkinnedMeshComponent.SetSkinnedAssetAndUpdate` (`self.Mesh`) Body true)
  (`SkinnedMeshComponent.SetSkinnedAssetAndUpdate` (`self.Head`) Head true)
  (`SkinnedMeshComponent.SetSkinnedAssetAndUpdate` (`self.Hair`) Hair true)
  (`SkinnedMeshComponent.SetSkinnedAssetAndUpdate` (`self.Hands`) Hands true)
  (`SkinnedMeshComponent.SetSkinnedAssetAndUpdate` (`self.Foot`) Foot true)
  (`SkinnedMeshComponent.SetSkinnedAssetAndUpdate` (`self.Legs`) Legs true))

(fn `ReinitBurst`
  (params (IsBursting :type Boolean))
  (returns (UpdatedWeaponInfo :type "WeaponInfo Structure"))
  (bind (_weaponclass _weaponname _canuseslot _rateoffire _reloadtime _maxround _currentround _burstfire _numberprojectilebyshot _burstrate _weaponrarity _dispersionweapon _soundfireweapon _soundreloadweapon _soundemptymagfire _effectfireweapon _projectilesetting _weapondamage _distacnetrace _decalonhit _shell _magazin _animweaponinfo _switchtimetoweapon _weaponicon _weapontype _weaponmesh) (break `WeaponInfo` (`self.WeaponSettings`)))
  (return (make `WeaponInfo` _weaponclass _weaponname _canuseslot _rateoffire _reloadtime _maxround _currentround IsBursting _numberprojectilebyshot _burstrate _dispersionweapon _soundfireweapon _soundreloadweapon _soundemptymagfire _effectfireweapon _projectilesetting _weapondamage _distacnetrace _decalonhit _shell _magazin _animweaponinfo _switchtimetoweapon _weaponicon _weapontype _weaponmesh)))

(fn `UserConstructionScript`
  (bind _mainweapon (`self.MainWeapon`))
  (if (`self.EquipedWeapon`)
    (`SceneComponent.SetVisibility` _mainweapon true false)
    (else
      (`SceneComponent.SetVisibility` _mainweapon false false)))
  (if (`self.isMale`)
    (`self.Init Outlook` "/Game/CharacterMeshes/MainMale/Meshes/Characters/Separates/TopBodies/SK_TopBody_A.SK_TopBody_A" "/Game/CharacterMeshes/MainMale/Meshes/Characters/Separates/Heads/SK_Head.SK_Head" "/Game/CharacterMeshes/MainMale/Meshes/Characters/Separates/Hairs/SK_Hair_C.SK_Hair_C" "/Game/CharacterMeshes/MainMale/Meshes/Characters/Separates/Hands/SK_Hands_JacketA.SK_Hands_JacketA" "/Game/CharacterMeshes/MainMale/Meshes/Characters/Separates/Shoes/SK_FabricShoesC4.SK_FabricShoesC4" "/Game/CharacterMeshes/MainMale/Meshes/Characters/Separates/BotBodies/SK_JeanPant_AC2.SK_JeanPant_AC2")
    (else
      (`self.Init Outlook` "/Game/CharacterMeshes/MainFemale/Meshes/Characters/Separates/TopBody/SK_TopBody_02.SK_TopBody_02" "/Game/CharacterMeshes/MainFemale/Meshes/Characters/Separates/Head/SK_HeadMakeUp.SK_HeadMakeUp" "/Game/CharacterMeshes/MainFemale/Meshes/Characters/Separates/Hairs/SK_HairS2_02.SK_HairS2_02" "/Game/CharacterMeshes/MainFemale/Meshes/Characters/Separates/Hands/SK_Hands.SK_Hands" "/Game/CharacterMeshes/MainFemale/Meshes/Characters/Separates/Shoes/SK_LeatherShoes.SK_LeatherShoes" "/Game/CharacterMeshes/MainFemale/Meshes/Characters/Separates/BotBody/SK_BotBody_02.SK_BotBody_02")))
  (`SkinnedMeshComponent.SetLeaderPoseComponent` (`self.Legs`) (`self.Mesh`) false)
  (`SkinnedMeshComponent.SetLeaderPoseComponent` (`self.Hands`) (`self.Mesh`) false)
  (`SkinnedMeshComponent.SetLeaderPoseComponent` (`self.Foot`) (`self.Mesh`) false)
  (`SkinnedMeshComponent.SetLeaderPoseComponent` (`self.Hair`) (`self.Mesh`) false)
  (`SkinnedMeshComponent.SetLeaderPoseComponent` (`self.Head`) (`self.Mesh`) false)
  (`SkinnedMeshComponent.SetLeaderPoseComponent` (`self.Accessory`) (`self.Mesh`) false)
  (`SkinnedMeshComponent.SetLeaderPoseComponent` (`self.SkeletalMesh`) (`self.Mesh`) false))