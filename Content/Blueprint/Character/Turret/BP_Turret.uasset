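; BP_Turret is a turret Blueprint whose SpinPart component sweeps back and forth in yaw.
; BeginPlay starts a fast looping timer that drives the sweep in place of Tick.
; Each timer call nudges the relative yaw by a fixed step, and the IsPositive flag flips direction once the rotation passes either limit of a symmetric arc.
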(event `CustomEvent_0`
  (bind (_relativerotation_roll _relativerotation_pitch _relativerotation_yaw) (`KismetMathLibrary.BreakRotator` (`SceneComponent.RelativeRotation` (`self.SpinPart`))))
  ;[1 1 1] GunSpin
  (if (`self.IsPositive`)
    (if (<= _relativerotation_yaw 50.0)
      (`SceneComponent.K2_AddRelativeRotation` (`self.SpinPart`) (struct :`Yaw` 1.0) false false)
      (else
        (set `self.IsPositive` false)))
    (elif (>= _relativerotation_yaw -50.0)
      (`SceneComponent.K2_AddRelativeRotation` (`self.SpinPart`) (struct :`Yaw` -1.0) false false)
      (else
        (set `self.IsPositive` true)))))

(event `self.ReceiveBeginPlay`
  ;[1 1 1] GunSpin
  (`KismetSystemLibrary.K2_SetTimerDelegate` (delegate `CustomEvent_0`) 0.02 true))

(event `self.ReceiveTick`
  (params (DeltaSeconds :type "Float (single-precision)")))

(fn `UserConstructionScript`)