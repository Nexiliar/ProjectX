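; Player character Blueprint for a top-down shooter, linking health, stats, inventory, weapon animations and HUD widgets.
; Inventory and stats load from PlayerState on BeginPlay and save back on unpossess; death requests a respawn or shows the end screen.
; Timer-stepped wheel zoom and cursor-led aim offset drive the camera, while damage adds blood decals and material blood.
; Prototype debug keys and hardcoded interaction remain, partly marked for removal.
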(event `self.CharHealthComponent.OnShieldChange`
  (params (Shield :type "Float (single-precision)") (Damage :type "Float (single-precision)")))

(event `self.CharHealthComponent.OnHealthChange`
  (params (Health :type "Float (single-precision)") (Damage :type "Float (single-precision)"))
  (bind _mesh (`self.Mesh`))
  (bind _returnvalue (`PrimitiveComponent.GetMaterial` _mesh 0))
  ;[1 1 1] DrawDecal
  (`|ExecutionSequence`
    (:`then_0`
      (if (< Damage 0.0)
        (if (> (`KismetMathLibrary.RandomFloat`) 0.6)
          (`GameplayStatics.SpawnDecalAtLocation` (select `int` (`KismetMathLibrary.RandomIntegerInRange` 0 2) :`0` "/Game/MS_Blood/Decal/010_Blood_Stain_sgfjdepc/010_Blood_Stain_sgfjdepc_8K_inst.010_Blood_Stain_sgfjdepc_8K_inst" :`1` "/Game/MS_Blood/Decal/02_Blood_Stain_sg3bdgoc/02_Blood_Stain_sg3bdgoc_8K_inst.02_Blood_Stain_sg3bdgoc_8K_inst" :`2` "/Game/MS_Blood/Decal/14_High_Velocity_Blood_Spatter_sgepbixp/14_High_Velocity_Blood_Spatter_sgepbixp_8K_inst.14_High_Velocity_Blood_Spatter_sgepbixp_8K_inst" :!type "MaterialInterface Object Reference") (30.0 60.0 60.0) (+ (`self.K2_GetActorLocation`) (`KismetMathLibrary.MakeVector` (`KismetMathLibrary.RandomFloatInRange` -32.0 32.0) (`KismetMathLibrary.RandomFloatInRange` -32.0 32.0) -120.0)) (struct :`Pitch` -90.0) 20.0))))
    (:`then_1`
      (bind _returnvalue_2 (`ProjectXHealthComponent.GetCurrentMaxHealth` (`self.CharHealthComponent`)))
      ;[1 1 1] Взаимодействие с динамическим материалом
      (bind _asmaterial_instance_dynamic (cast `MaterialInstanceDynamic` _returnvalue)
        (:`then`
          (bind _returnvalue_3 (`KismetMathLibrary.MapRangeClamped` Health (- _returnvalue_2 60.0) _returnvalue_2 1.0 0.2))
          (`MaterialInstanceDynamic.SetScalarParameterValue` _asmaterial_instance_dynamic "Blood" _returnvalue_3))
        (:`CastFailed`
          (bind _returnvalue_4 (`PrimitiveComponent.CreateDynamicMaterialInstance` _mesh 0 _returnvalue "BloodyDynamic"))
          (`MaterialInstanceDynamic.SetScalarParameterValue` _returnvalue_4 "Blood" _returnvalue_3)
          (`PrimitiveComponent.SetMaterial` _mesh 0 _returnvalue_4))))))

(event `AddExp`
  (bind _statscomponent (`self.StatsComponent`))
  ;[1 1 1] EXP ADD
  (bind _asbp_player_state (cast `/Game/Blueprint/Game/BP_PlayerState` (`self.PlayerState`)))
  (`ProjectXStatsComponent.ExpGain` _statscomponent (`/Game/Blueprint/Game/BP_PlayerState.Exp` _asbp_player_state))
  (bind (_currentmaxexp _returnvalue) (`ProjectXStatsComponent.GetExpInfo` _statscomponent))
  (bind _asbp_player_controller (cast `/Game/Blueprint/Game/BP_PlayerController` (`GameplayStatics.GetPlayerController` 0)))
  (`/Game/Blueprint/Widget/Stats/W_Stats.Stats Exp` (`/Game/Blueprint/Widget/W_Ingame.W_Stats` (`/Game/Blueprint/Game/BP_PlayerController.IngameWidget` _asbp_player_controller)) _returnvalue _currentmaxexp))

(event `Key|B`
  (params (Key :type "Key Structure"))
  (:`Pressed`
    (`ProjectXStatsComponent.ExpGain` (`self.StatsComponent`) 5000.0)
    (`KismetSystemLibrary.PrintString` "addexp")))

(event `self.WeaponReloadStart_BP`
  (params (Anim :type "AnimMontage Object Reference"))
  ;[1 1 1] CharacterAnimations
  (`/Game/Blueprint/Character/Mannequin/Animations/ThirdPerson_AnimBP.Reload` (`self.AnimInstance`) Anim)
  (bind _asbp_player_controller (cast `/Game/Blueprint/Game/BP_PlayerController` (`self.GetController`)))
  (bind _ingamewidget (`/Game/Blueprint/Game/BP_PlayerController.IngameWidget` _asbp_player_controller))
  (`/Engine/EditorBlueprintResources/StandardMacros.IsValid` _ingamewidget
    (:`Is Valid`
      (`/Game/Blueprint/Widget/Inventory/W_InventoryStats.WeaponReloadStart` (`/Game/Blueprint/Widget/W_Ingame.W_InventoryStats` _ingamewidget)))))

(event `self.WeaponFireStart_BP`
  (params (Anim :type "AnimMontage Object Reference"))
  ;[1 1 1] CharacterAnimations
  (`/Game/Blueprint/Character/Mannequin/Animations/ThirdPerson_AnimBP.Fire` (`self.AnimInstance`) Anim))

(event `self.WeaponReloadEnd_BP`
  (params (bIsSucces :type Boolean))
  ;[1 1 1] CharacterAnimations
  (`/Game/Blueprint/Character/Mannequin/Animations/ThirdPerson_AnimBP.ReloadEnd` (`self.AnimInstance`) bIsSucces)
  (bind _asbp_player_controller (cast `/Game/Blueprint/Game/BP_PlayerController` (`self.GetController`)))
  (bind _ingamewidget (`/Game/Blueprint/Game/BP_PlayerController.IngameWidget` _asbp_player_controller))
  (`/Engine/EditorBlueprintResources/StandardMacros.IsValid` _ingamewidget
    (:`Is Valid`
      (`/Game/Blueprint/Widget/Inventory/W_InventoryStats.WeaponReloadEnd` (`/Game/Blueprint/Widget/W_Ingame.W_InventoryStats` _ingamewidget) bIsSucces))))

(event `self.CharDead_BP`
  ;[1 1 1] Comment
  (`PrimitiveComponent.SetCollisionResponseToChannel` (`self.CapsuleComponent`) "ECC_Pawn" "ECR_Ignore")
  (`PrimitiveComponent.SetCollisionResponseToChannel` (`self.Mesh`) "ECC_Pawn" "ECR_Ignore")
  (`PrimitiveComponent.SetCollisionResponseToChannel` (`self.BackPack`) "ECC_Pawn" "ECR_Ignore")
  (`PrimitiveComponent.SetCollisionResponseToChannel` (`self.Armor`) "ECC_Pawn" "ECR_Ignore")
  (`PrimitiveComponent.SetCollisionResponseToChannel` (`self.Pistol`) "ECC_Pawn" "ECR_Ignore")
  (bind _returnvalue (`self.GetCurrentWeapon`))
  (`/Engine/EditorBlueprintResources/StandardMacros.IsValid` _returnvalue
    (:`Is Valid`
      (`self.SetLifeSpan` _returnvalue 20.0))
    (:`Is Not Valid`
      _))
  (`self.SetLifeSpan` 20.0)
  (bind _asbp_main_game_mode (cast `/Game/Blueprint/Game/BP_MainGameMode` (`GameplayStatics.GetGameMode`)))
  (bind _succes (`/Game/Blueprint/Game/BP_MainGameMode.RespawnPlayerAtPoint` _asbp_main_game_mode null))
  (if (not _succes)
    (bind _returnvalue_2 (`|CreateWidget` "/Game/Blueprint/Widget/Menu/W_EndGame.W_EndGame_C"))
    (`UserWidget.AddToViewport` _returnvalue_2 0)
    (set `PlayerController.bShowMouseCursor` true (`GameplayStatics.GetPlayerController` 0))))

(event `self.ReceiveBeginPlay`
  ;[1 1 1] BeginPlay
  (bind _asthird_person_anim_bp (cast `/Game/Blueprint/Character/Mannequin/Animations/ThirdPerson_AnimBP` (`SkeletalMeshComponent.GetAnimInstance` (`self.Mesh`))))
  (set `self.AnimInstance` _asthird_person_anim_bp)
  (`|ExecutionSequence`
    (:`then_0`
      (`self.PlayerInitialization`))
    (:`then_1`
      ;[1 1 1] ItemUseLogic
      (add `ProjectXInventoryComponent.OnItemUsed` (`self.InventoryComponent`) (delegate `CustomEvent_0`)))
    (:`then_2`
      (`KismetSystemLibrary.K2_SetTimerDelegate` (delegate `ItemDropCoords`) 0.1 true))))

(event `self.ReceiveUnpossessed`
  (params (OldController :type "Controller Object Reference"))
  (bind _inventorycomponent (`self.InventoryComponent`))
  ;[1 1 1] Comment
  (bind _asbp_player_state (cast `/Game/Blueprint/Game/BP_PlayerState` (`Controller.PlayerState` OldController)))
  (`/Game/Blueprint/Game/BP_PlayerState.SaveCurrentInventory` _asbp_player_state (`ProjectXInventoryComponent.AmmoSlots` _inventorycomponent) (`ProjectXInventoryComponent.WeaponSlotsInfo` _inventorycomponent))
  (bind (_level _skillpoints _att _returnvalue) (`ProjectXStatsComponent.GetEveryStat` (`self.StatsComponent`)))
  (`/Game/Blueprint/Game/BP_PlayerState.SaveCurrentStats` _asbp_player_state _level _skillpoints _att _returnvalue)
  (bind _asbp_player_controller (cast `/Game/Blueprint/Game/BP_PlayerController` OldController))
  (`/Game/Blueprint/Widget/Inventory/W_InventoryStats.UnbindAllEvents` (`/Game/Blueprint/Widget/W_Ingame.W_InventoryStats` (`/Game/Blueprint/Game/BP_PlayerController.IngameWidget` _asbp_player_controller)) self)
  (bind _maininventoryingamewidget (`/Game/Blueprint/Game/BP_PlayerController.MainInventoryIngameWidget` _asbp_player_controller))
  (`/Game/Blueprint/Widget/Stats/W_MainCharacterStats.UnbindEvent` (`/Game/Blueprint/Widget/Inventory/InventorySystem/W_MainScreenWidget.W_MainCharacterStats` _maininventoryingamewidget))
  (`/Game/Blueprint/Widget/Inventory/InventorySystem/W_MainCharacterWidget.UnbindAllEvents` (`/Game/Blueprint/Widget/Inventory/InventorySystem/W_MainScreenWidget.W_MainCharacterWidget` _maininventoryingamewidget)))

(event `CustomEvent_0`
  (params (AmountOfItemsToUse :type Integer) (InventorySlotInfo :type "Inventory Structure"))
  ;[1 1 1] ItemUseLogic
  (`|ExecutionSequence`
    (:`then_0`
      (if (== (break `ItemsInfo` (break `Inventory` InventorySlotInfo)) "AmmoPack")
        (if (`ProjectXInventoryComponent.isBodyKitEquiped` (`self.InventoryComponent`))
          (for (_array_element _array_index) (`ProjectXInventoryComponent.AmmoSlots` (`self.InventoryComponent`))
            (bind (_weapontype _count _maxcount) (break `AmmoSlot` _array_element))
            (bind _returnvalue (+ _count 20))
            (if (>= _returnvalue _maxcount)
              (`KismetArrayLibrary.Array_Set` (`ProjectXInventoryComponent.AmmoSlots` (`self.InventoryComponent`)) _array_index (make `AmmoSlot` _weapontype _maxcount _maxcount))
              (else
                (`KismetArrayLibrary.Array_Set` (`ProjectXInventoryComponent.AmmoSlots` (`self.InventoryComponent`)) _array_index (make `AmmoSlot` _weapontype _returnvalue _maxcount))))
            (`self.OnAmmoPackUse`)))))
    (:`then_1`
      (if (== (break `ItemsInfo` (break `Inventory` InventorySlotInfo)) "HealthPack")
        (`ProjectXCharacterHealthComponent.HealthRegenStart` (`self.CharHealthComponent`) 20.0)))))

(event `ItemDropCoords`
  (set `ProjectXInventoryComponent.VariableToSpawnEquip` (`SceneComponent.GetSocketLocation` (`self.Mesh`) "SpawnItemSocket") (`self.InventoryComponent`)))

(event `InputAction|Inventory`
  (params (Key :type "Key Structure"))
  ;[0 0.2447 1] InventoryCall
  (:`Pressed`
    (bind _asbp_player_controller (cast `/Game/Blueprint/Game/BP_PlayerController` (`self.GetController`)))
    (bind _maininventoryingamewidget (`/Game/Blueprint/Game/BP_PlayerController.MainInventoryIngameWidget` _asbp_player_controller))
    (`/Game/Blueprint/Widget/Inventory/InventorySystem/W_MainScreenWidget.ShowHideInventory` _maininventoryingamewidget)
    (`/Engine/EditorBlueprintResources/StandardMacros.DoOnce` false
      (:`Completed`
        (bind _w_inventory (`/Game/Blueprint/Widget/Inventory/InventorySystem/W_MainScreenWidget.W_Inventory` _maininventoryingamewidget))
        (`/Engine/EditorBlueprintResources/StandardMacros.IsValid` _w_inventory
          (:`Is Valid`
            (`/Game/Blueprint/Widget/Inventory/InventorySystem/W_Inventory.TryToBuildIn` _w_inventory))
          (:`Is Not Valid`
            _))
        (bind _w_maincharacterstats (`/Game/Blueprint/Widget/Inventory/InventorySystem/W_MainScreenWidget.W_MainCharacterStats` _maininventoryingamewidget))
        (`/Engine/EditorBlueprintResources/StandardMacros.IsValid` _w_maincharacterstats
          (:`Is Valid`
            (`/Game/Blueprint/Widget/Stats/W_MainCharacterStats.TryToBuildStats` _w_maincharacterstats)))))))

(event `self.ReceiveTick`
  (params (DeltaSeconds :type "Float (single-precision)"))
  (bind _inventorycomponent (`self.InventoryComponent`))
  (bind _armor (`self.Armor`))
  (`|ExecutionSequence`
    (:`then_0`
      ;[1 1 1] Delete after REDONE
      (`self.CameraAimFunc` DeltaSeconds))
    (:`then_1`
      (if (`ProjectXInventoryComponent.isBackPackEquiped` _inventorycomponent)
        (`SceneComponent.SetVisibility` (`self.BackPack`) true false)
        (else
          (`SceneComponent.SetVisibility` (`self.BackPack`) false false))))
    (:`then_2`
      (if (`ProjectXInventoryComponent.isArmorEquiped` _inventorycomponent)
        (`SceneComponent.SetVisibility` _armor true false)
        (else
          (`SceneComponent.SetVisibility` _armor false false))))))

(event `InputAction|Walking`
  (params (Key :type "Key Structure"))
  ;[0 1 0.1258] MovementState Logic
  (:`Pressed`
    (set `self.WalkEnabled` true)
    (`self.ChangeMovementState` :!label _label))
  (:`Released`
    (set `self.WalkEnabled` false)
    (goto _label)))

(event `Key|Y`
  (params (Key :type "Key Structure")))

(event `Key|F`
  (params (Key :type "Key Structure"))
  ;[1 1 1] CameraLogic
  (:`Pressed`
    (`self.CameraShakeEvent`)))

(event `InputAction|Sprint`
  (params (Key :type "Key Structure"))
  ;[0 1 0.1258] MovementState Logic
  (:`Pressed`
    (set `self.SprintCheck` true)
    (goto _label))
  (:`Released`
    (set `self.SprintCheck` false)
    (goto _label)))

(event `Key|H`
  (params (Key :type "Key Structure"))
  (bind _weaponslotsinfo (`ProjectXInventoryComponent.WeaponSlotsInfo` (`self.InventoryComponent`)))
  ;[1 0.05156 0.04161] Прототип функции открытия доступа к закрытым слотам удалить, после реворка в с++
  (:`Pressed`
    (for (_ _array_index) _weaponslotsinfo
      (if (not true)
        (bind (_weaponclass _weaponname _canuseslot _rateoffire _reloadtime _maxround _currentround _burstfire _numberprojectilebyshot _burstrate _dispersionweapon _soundfireweapon _soundreloadweapon _soundemptymagfire _effectfireweapon _projectilesetting _weapondamage _distacnetrace _decalonhit _shell _magazin _animweaponinfo _switchtimetoweapon _weaponicon _weapontype _weaponmesh) (break `WeaponInfo` (`|GetArrayItem` _weaponslotsinfo _array_index)))
        (`KismetArrayLibrary.Array_Set` _weaponslotsinfo _array_index (make `WeaponInfo` _weaponclass _weaponname true _rateoffire _reloadtime _maxround _currentround false _numberprojectilebyshot 0.1 _dispersionweapon _soundfireweapon _soundreloadweapon _soundemptymagfire _effectfireweapon _projectilesetting _weapondamage _distacnetrace _decalonhit _shell _magazin _animweaponinfo _switchtimetoweapon _weaponicon _weapontype _weaponmesh))
        (break)))))

(event `InputAxis|MouseWheel`
  (params (AxisValue :type "Float (single-precision)"))
  ;[1 1 1] CameraLogic
  (`self.CameraSlide` AxisValue))

(event `InputAction|Aim`
  (params (Key :type "Key Structure"))
  ;[0 1 0.1258] MovementState Logic
  (:`Pressed`
    (if (`self.IsArmed`)
      (set `self.AimEnabled` true)
      (goto _label)))
  (:`Released`
    (set `self.AimEnabled` false)
    (goto _label)))

(event `InputAction|Crouch`
  (params (Key :type "Key Structure"))
  ;[0 1 0.1258] MovementState Logic
  (:`Pressed`
    (set `self.CrouchEnabled` true)
    (goto _label))
  (:`Released`
    (set `self.CrouchEnabled` false)
    (goto _label)))

(event `Key|Y`
  (params (Key :type "Key Structure"))
  (:`Pressed`
    (`ProjectXInventoryComponent.SetAmmoInBodyKit` (`self.InventoryComponent`) "Rifle" 50)))

(event `Key|E`
  (params (Key :type "Key Structure"))
  ;[1 1 1] Old Interact sys? Del after rework
  (:`Pressed`
    (if (`self.isCloseToButton`)
      (bind _returnvalue (`GameplayStatics.GetActorOfClass` "/Game/Blueprint/Game/Props/BP_SmallGate.BP_SmallGate_C"))
      (`/Game/Blueprint/Game/Props/BP_SmallGate.TimerGO` _returnvalue)
      (bind _returnvalue_2 (`GameplayStatics.GetActorOfClass` "/Game/Blueprint/Game/Props/BP_TopLight.BP_TopLight_C"))
      (`/Game/Blueprint/Game/Props/BP_TopLight.Available` _returnvalue_2)
      (elif (`self.isCloseToPick`)
        (bind _returnvalue_3 (`GameplayStatics.GetActorOfClass` "/Game/Blueprint/Game/Props/BP_Card.BP_Card_C"))
        (set `self.haveACard` true)
        (`self.K2_DestroyActor` _returnvalue_3)
        (elif (`self.isCloseSecurityTerminal`)
          (bind _outactors (`GameplayStatics.GetAllActorsOfClass` "/Game/Blueprint/Game/Props/BP_GateT.BP_GateT_C"))
          (`/Game/Blueprint/Game/Props/BP_GateT.Available` (`|GetArrayItem` _outactors 5)))))))

(fn `CameraAimFunc`
  (params (float :type "Float (double-precision)"))
  (bind _cameraboom (`self.CameraBoom`))
  (bind _movementstate (`self.MovementState`))
  (bind _returnvalue (`SceneComponent.K2_GetComponentLocation` (`self.CapsuleComponent`)))
  (bind (_returnvalue_x _returnvalue_y _returnvalue_z) (`KismetMathLibrary.BreakVector` (`SceneComponent.K2_GetComponentLocation` (`self.CameraBoom`))))
  ;[1 1 1] AIM
  (bind _returnvalue_2 (`self.GetCursorToWorld`))
  (set `self.ClampedCameraHeight` (`KismetMathLibrary.MapRangeClamped` (`SpringArmComponent.TargetArmLength` (`self.CameraBoom`)) (`self.HeightCameraMin`) (`self.HeightCameraMax`) 0.5 1.0))
  (bind _returnvalue_3 (`SceneComponent.K2_GetComponentLocation` _returnvalue_2))
  (set `self.DistanceCameraBoom` (`KismetMathLibrary.VSizeXY` (- _returnvalue _returnvalue_3)))
  (if (or (`|EnumEquality` _movementstate "Aim_State") (`|EnumEquality` _movementstate "AimWalk_State") (`|EnumEquality` _movementstate "AimCrouch_State"))
    (if (> (`self.DistanceCameraBoom`) (* (`self.ClampedCameraHeight`) (`self.F Min Clamp Distance Logic`)))
      (if (not (> (`KismetMathLibrary.VSize2D` (`KismetMathLibrary.Conv_VectorToVector2D` (- (`SceneComponent.K2_GetComponentLocation` (`self.CameraBoom`)) _returnvalue))) (* (`self.ClampedCameraHeight`) (`self.F Max Clamp Distance Logic`))))
        (bind (_x _y) (`KismetMathLibrary.BreakVector2D` (* (`KismetMathLibrary.Normal2D` (`KismetMathLibrary.Conv_VectorToVector2D` (`KismetMathLibrary.GetForwardVector` (`KismetMathLibrary.FindLookAtRotation` _returnvalue _returnvalue_3)))) (`self.FSpeedChangeLocationCameratoCursor`))))
        (`SceneComponent.K2_SetWorldLocation` (`self.CameraBoom`) (`KismetMathLibrary.MakeVector` (+ _x _returnvalue_x) (+ _y _returnvalue_y) _returnvalue_z) false false))
      (else
        (`SceneComponent.K2_SetWorldLocation` _cameraboom (`KismetMathLibrary.VInterpTo` (`SceneComponent.K2_GetComponentLocation` _cameraboom) (`SceneComponent.K2_GetComponentLocation` (`self.CapsuleComponent`)) float (`self.FSpeedReturnCameraDefaultPosition`)) false false :!label _label)))
    (else
      (goto _label))))

(fn `CameraShakeEvent`
  (`GameplayStatics.PlayWorldCameraShake` "/Game/Blueprint/Game/BP_ShakeCamera.BP_ShakeCamera_C" (`SceneComponent.K2_GetComponentLocation` (`self.TopDownCameraComponent`)) 0.0 30.0))

(fn `CameraSlide`
  (params (Value :type "Float (double-precision)"))
  (bind (_rotationcamera_roll _rotationcamera_pitch) (`KismetMathLibrary.BreakRotator` (`self.RotationCamera`)))
  (bind (_rotationcamera_roll_2 _rotationcamera_pitch_2) (`KismetMathLibrary.BreakRotator` (`self.RotationCamera`)))
  (bind _returnvalue (- _rotationcamera_pitch_2 3.0))
  (bind _returnvalue_2 (+ _rotationcamera_pitch 2.5))
  (if (`self.SlideDone`)
    (if (!= Value 0.0)
      (if (< Value 0.0)
        (if (not (<= _rotationcamera_pitch_2 -60.0))
          (`SceneComponent.K2_SetRelativeRotation` (`self.CameraBoom`) (`KismetMathLibrary.MakeRotator` 0.0 _returnvalue) false false)
          (set `self.RotationCamera` (`KismetMathLibrary.MakeRotator` 0.0 _returnvalue))
          (if (>= (`self.HeightCameraMax`) (+ (`SpringArmComponent.TargetArmLength` (`self.CameraBoom`)) (`self.HeightCameraCHangeDIstance`)))
            (set `self.SlideUp` true)
            (set `self.SlideDone` false :!label _label)
            (bind _returnvalue_3 (`KismetSystemLibrary.K2_SetTimer` null "CameraSlideSmoth" (`self.TimerStep`) true))
            (set `self.SlideTimer` _returnvalue_3)))
        (elif (not (>= _rotationcamera_pitch -38.0))
          (`SceneComponent.K2_SetRelativeRotation` (`self.CameraBoom`) (`KismetMathLibrary.MakeRotator` 0.0 _returnvalue_2) false false)
          (set `self.RotationCamera` (`KismetMathLibrary.MakeRotator` 0.0 _returnvalue_2))
          (if (<= (`self.HeightCameraMin`) (- (`SpringArmComponent.TargetArmLength` (`self.CameraBoom`)) (`self.HeightCameraCHangeDIstance`)))
            (set `self.SlideUp` false)
            (goto _label)))))))

(fn `CameraSlideSmoth`
  (bind _heightcamerachangeslidestepdistance (`self.HeightCameraChangeSlideStepDistance`))
  (bind _targetarmlength (`SpringArmComponent.TargetArmLength` (`self.CameraBoom`)))
  (bind _output_get (set `self.CurrentSlideDistance` (+ (`self.HeightCameraChangeSlideStepDistance`) (`self.CurrentSlideDistance`))))
  (set `SpringArmComponent.TargetArmLength` (select `bool` (`self.SlideUp`) :`false` (- _targetarmlength _heightcamerachangeslidestepdistance) :`true` (+ _targetarmlength _heightcamerachangeslidestepdistance)) (`self.CameraBoom`))
  (if (>= _output_get (`self.HeightCameraCHangeDIstance`))
    (set `self.CurrentSlideDistance` 0.0)
    (set `self.SlideDone` true)
    (`KismetSystemLibrary.K2_ClearAndInvalidateTimerHandle` (`self.SlideTimer`))))

(fn `PlayerInitialization`
  (bind _returnvalue (`GameplayStatics.GetPlayerController` 0))
  (`|ExecutionSequence`
    (:`then_0`
      (bind _asbp_player_state (cast `/Game/Blueprint/Game/BP_PlayerState` (`Controller.PlayerState` _returnvalue)))
      (`ProjectXInventoryComponent.InitInventory` (`self.InventoryComponent`) (`/Game/Blueprint/Game/BP_PlayerState.WeaponSlots` _asbp_player_state) (`/Game/Blueprint/Game/BP_PlayerState.AmmoSlots` _asbp_player_state))
      (bind _asbp_player_controller (cast `/Game/Blueprint/Game/BP_PlayerController` _returnvalue))
      (bind _ingamewidget (`/Game/Blueprint/Game/BP_PlayerController.IngameWidget` _asbp_player_controller))
      (`/Game/Blueprint/Widget/Inventory/W_InventoryStats.InitInventoryStatsWidget` (`/Game/Blueprint/Widget/W_Ingame.W_InventoryStats` _ingamewidget) self)
      (`/Game/Blueprint/Widget/Health/W_StatsCharacterBar.InitWidget` (`/Game/Blueprint/Widget/W_Ingame.W_HealthBar` _ingamewidget))
      (bind _maininventoryingamewidget (`/Game/Blueprint/Game/BP_PlayerController.MainInventoryIngameWidget` _asbp_player_controller))
      (`/Game/Blueprint/Widget/Inventory/InventorySystem/W_MainCharacterWidget.MainCharacterWidgetInit` (`/Game/Blueprint/Widget/Inventory/InventorySystem/W_MainScreenWidget.W_MainCharacterWidget` _maininventoryingamewidget))
      (`/Game/Blueprint/Widget/Stats/W_MainCharacterStats.PlayerStatsInit` (`/Game/Blueprint/Widget/Inventory/InventorySystem/W_MainScreenWidget.W_MainCharacterStats` _maininventoryingamewidget)))
    (:`then_1`
      (`ProjectXStatsComponent.StatsInit` (`self.StatsComponent`) (`/Game/Blueprint/Game/BP_PlayerState.PlayerLevel` _asbp_player_state) (`/Game/Blueprint/Game/BP_PlayerState.PlayerSkillPoints` _asbp_player_state) (`/Game/Blueprint/Game/BP_PlayerState.PlayerAttributePoints` _asbp_player_state) (`/Game/Blueprint/Game/BP_PlayerState.StatsInfo` _asbp_player_state)))))

(fn `Sprint`)

(fn `UserConstructionScript`
  (set `SpringArmComponent.TargetArmLength` (`self.HeightCameraMax`) (`self.CameraBoom`))
  (`SceneComponent.K2_SetRelativeRotation` (`self.CameraBoom`) (`self.RotationCamera`) false false)
  (set `SpringArmComponent.bEnableCameraLag` (`self.Flow`) (`self.CameraBoom`))
  (set `SpringArmComponent.CameraLagSpeed` (`self.CoefSmoth`) (`self.CameraBoom`)))