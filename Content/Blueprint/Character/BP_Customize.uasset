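; BP_Customize is a modular character body that dresses itself as male or female from the IsMale flag.
; On BeginPlay it assigns skeletal meshes for top body, legs, feet, head, hair and hands, with both branches using the same hands mesh.
; The construction script makes legs, hands, head and feet follow Mesh through master pose, leaving hair out.
; Two looping idle animation calls are left unconnected.
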(event `self.ReceiveBeginPlay`
  (bind _sk_legs (`self.SK_Legs`))
  (bind _mesh (`self.Mesh`))
  (bind _sk_foot (`self.SK_Foot`))
  (bind _sk_head (`self.SK_Head`))
  (bind _sk_hair (`self.SK_Hair`))
  (bind _sk_hands (`self.SK_Hands`))
  (if (`self.isMale?`)
    (`SkinnedMeshComponent.SetSkinnedAssetAndUpdate` _mesh "/Game/CharacterMeshes/MainMale/Meshes/Characters/Separates/TopBodies/SK_TopBody.SK_TopBody" true)
    (`SkinnedMeshComponent.SetSkinnedAssetAndUpdate` _sk_legs "/Game/CharacterMeshes/MainMale/Meshes/Characters/Separates/BotBodies/SK_BotBody.SK_BotBody" true)
    (`SkinnedMeshComponent.SetSkinnedAssetAndUpdate` _sk_foot "/Game/CharacterMeshes/MainMale/Meshes/Characters/Separates/Shoes/SK_Feet.SK_Feet" true)
    (`SkinnedMeshComponent.SetSkinnedAssetAndUpdate` _sk_head "/Game/CharacterMeshes/MainMale/Meshes/Characters/Separates/Heads/SK_Head.SK_Head" true)
    (`SkinnedMeshComponent.SetSkinnedAssetAndUpdate` _sk_hair "/Game/CharacterMeshes/MainMale/Meshes/Characters/Separates/Hairs/SK_Hair_A.SK_Hair_A" true)
    (`SkinnedMeshComponent.SetSkinnedAssetAndUpdate` _sk_hands "/Game/CharacterMeshes/MainMale/Meshes/Characters/Separates/Hands/SK_Hands.SK_Hands" true)
    (else
      (`SkinnedMeshComponent.SetSkinnedAssetAndUpdate` _mesh "/Game/CharacterMeshes/MainFemale/Meshes/Characters/Separates/TopBody/SK_TopBody_01.SK_TopBody_01" true)
      (`SkinnedMeshComponent.SetSkinnedAssetAndUpdate` _sk_legs "/Game/CharacterMeshes/MainFemale/Meshes/Characters/Separates/BotBody/SK_BotBody_01.SK_BotBody_01" true)
      (`SkinnedMeshComponent.SetSkinnedAssetAndUpdate` _sk_foot "/Game/CharacterMeshes/MainFemale/Meshes/Characters/Separates/Shoes/SK_Foots.SK_Foots" true)
      (`SkinnedMeshComponent.SetSkinnedAssetAndUpdate` _sk_head "/Game/CharacterMeshes/MainFemale/Meshes/Characters/Separates/Head/SK_HeadMakeUp.SK_HeadMakeUp" true)
      (`SkinnedMeshComponent.SetSkinnedAssetAndUpdate` _sk_hair "/Game/CharacterMeshes/MainFemale/Meshes/Characters/Separates/Hairs/SK_HairS2.SK_HairS2" true)
      (`SkinnedMeshComponent.SetSkinnedAssetAndUpdate` _sk_hands "/Game/CharacterMeshes/MainFemale/Meshes/Characters/Separates/Hands/SK_Hands.SK_Hands" true))))

(fn `UserConstructionScript`
  (`SkinnedMeshComponent.SetLeaderPoseComponent` (`self.SK_Legs`) (`self.Mesh`) false)
  (`SkinnedMeshComponent.SetLeaderPoseComponent` (`self.SK_Hands`) (`self.Mesh`) false)
  (`SkinnedMeshComponent.SetLeaderPoseComponent` (`self.SK_Head`) (`self.Mesh`) false)
  (`SkinnedMeshComponent.SetLeaderPoseComponent` (`self.SK_Foot`) (`self.Mesh`) false))