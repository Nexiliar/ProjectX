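; Fire state effect that shows the burning debuff and its timer on the player's in-game HUD.
; On BeginPlay it caches the player controller and binds to the debuff-time-started event.
; A DoOnce, re-armed when remaining time runs out, gates creation of the Fire icon in the buff/debuff widget.
; Each event also searches that widget's children for a debuff icon to pass the remaining and additional time.
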(event `self.BeginPlay`
  (bind _asbp_character (cast `/Game/Blueprint/Character/BP_Character` (`GameplayStatics.GetPlayerPawn` self)))
  (bind _asbp_player_controller (cast `/Game/Blueprint/Game/BP_PlayerController` (`GameplayStatics.GetPlayerController` _asbp_character)))
  (set `self.As BP Player Controller` _asbp_player_controller)
  (add `self.OnDebuffTimeStarted` (delegate `DebuffStarted`)))

(event `DebuffStarted` :!signature `self.OnDebuffTimeStarted`
  (params (TimeRemainingForWidget :type "Float (double-precision)") (AdditionalTimeRemainingForWidget :type "Float (double-precision)"))
  (bind _w_buff_debuff (`/Game/Blueprint/Widget/W_Ingame.W_Buff_Debuff` (`/Game/Blueprint/Game/BP_PlayerController.IngameWidget` (`self.As BP Player Controller`))))
  (`|ExecutionSequence`
    (:`then_0`
      (if (<= TimeRemainingForWidget 0.0)
        (goto _label :!via `Reset`)
        (else
          (`/Engine/EditorBlueprintResources/StandardMacros.DoOnce` false :!label _label
            (:`Completed`
              (`/Game/Blueprint/Widget/Buff_Debuff/W_Buff_Debuff.DebufInit` _w_buff_debuff "Fire"))))))
    (:`then_1`
      (for _array_element (`PanelWidget.GetAllChildren` (`/Game/Blueprint/Widget/Buff_Debuff/W_Buff_Debuff.VerticalBox_BuffLine` _w_buff_debuff))
        (bind _asw_de_buff_icon (cast `/Game/Blueprint/Widget/Buff_Debuff/W_DeBuffIcon` _array_element))
        (if (== _asw_de_buff_icon "/Game/Blueprint/Widget/Buff_Debuff/W_DeBuffIcon.W_DeBuffIcon")
          (break)))
      (`/Game/Blueprint/Widget/Buff_Debuff/W_DeBuffIcon.TimerCount` _asw_de_buff_icon TimeRemainingForWidget AdditionalTimeRemainingForWidget))))