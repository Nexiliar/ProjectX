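; BP_Bomb is a timed bomb projectile that explodes five seconds after spawning.
; On BeginPlay, a looping timer blinks its point light off and on each second as a countdown warning.
; A one-shot timer then applies radial damage with falloff at the Cube mesh's location, spawns a grenade explosion effect and sound, and destroys the actor.
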(event `self.ReceiveBeginPlay`
  (`KismetSystemLibrary.K2_SetTimerDelegate` (delegate `LightIntencityChange`) 1.0 true)
  (`KismetSystemLibrary.K2_SetTimerDelegate` (delegate `BombTimer`) 5.0))

(event `BombTimer`
  (bind _returnvalue (`SceneComponent.K2_GetComponentLocation` (`self.Cube`)))
  (`GameplayStatics.ApplyRadialDamageWithFalloff` :`BaseDamage` 200.0 :`MinimumDamage` 20.0 :`Origin` _returnvalue :`DamageInnerRadius` 200.0 :`DamageOuterRadius` 400.0 :`DamageFalloff` 0.5 :`DamageTypeClass` "/Script/Engine.DamageType" :`DamageCauser` null :`InstigatedByController` null)
  (`GameplayStatics.SpawnEmitterAtLocation` "/Game/Items/GameActor/Weapons/FX/P_Grenade_Explosion_01.P_Grenade_Explosion_01" _returnvalue (struct) (3.0 3.0 3.0))
  (`GameplayStatics.SpawnSoundAtLocation` "/Game/Items/GameActor/Weapons/Sound/GrenadeLauncher/Wavs/GrenadeLauncher_Explosion04.GrenadeLauncher_Explosion04" _returnvalue (struct) 1.0 1.0 0.0 null null)
  (`self.K2_DestroyActor`))

(event `LightIntencityChange`
  (bind _pointlight (`self.PointLight`))
  (`LightComponent.SetIntensity` _pointlight 0.0)
  (`KismetSystemLibrary.Delay` 0.5)
  (`LightComponent.SetIntensity` _pointlight 1000.0))

(fn `UserConstructionScript`)